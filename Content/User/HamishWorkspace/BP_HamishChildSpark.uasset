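; BP_HamishChildSpark is a child Blueprint of a controlled pawn, apparently the Spark, that adds a reset to a given position.
; ResetToSpecificPosition fades the camera out, ignores move input, then after a short delay teleports to the position with zero rotation.
; Only a successful teleport restores input, fades back in and calls OnResetToSafeLocationComplete; failure leaves the screen faded and movement locked.
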(event `ResetToSpecificPosition`
  (params (SpecificPosition :type "Vector Structure"))
  ;[1 1 1] Reset to specific location
  (`PlayerCameraManager.StartCameraFade` :`self` (`GameplayStatics.GetPlayerCameraManager` 0) :`ToAlpha` 1.0 :`Duration` 0.4 :`bHoldWhenFinished` true)
  (`Controller.SetIgnoreMoveInput` (`self.GetController`) true)
  (`KismetSystemLibrary.Delay` 0.8)
  (bind _returnvalue (`self.K2_TeleportTo` SpecificPosition))
  (if _returnvalue
    (`Controller.SetIgnoreMoveInput` (`self.GetController`) false)
    (`PlayerCameraManager.StartCameraFade` :`self` (`GameplayStatics.GetPlayerCameraManager` 0) :`FromAlpha` 1.0 :`Duration` 0.4 :`bHoldWhenFinished` true)
    (`self.OnResetToSafeLocationComplete`)))

(fn `UserConstructionScript`
  (`parent.UserConstructionScript`))